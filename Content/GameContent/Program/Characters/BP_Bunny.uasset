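; BP_Bunny is a bunny character Blueprint that shows either a male or a female bunny model.
; Its construction script runs the parent's script, then sets the AnimalMesh static mesh from the IsMale flag.
; The event graph holds only disabled default events, so the Blueprint adds no runtime logic of its own.
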(event EventBeginPlay
  (|CallParentFunction) ; This node is disabled and will not be called.\nDrag off pins to build functionality.
)

(event Collision|EventActorBeginOverlap
  (params (OtherActor :type Actor%20Object%20Reference))
  (|CallParentFunction OtherActor) ; This node is disabled and will not be called.\nDrag off pins to build functionality.
)

(event EventTick
  (params (DeltaSeconds :type Float%20%28single-precision%29))
  (|CallParentFunction DeltaSeconds) ; This node is disabled and will not be called.\nDrag off pins to build functionality.
)

(fn ConstructionScript
  (|CallParentFunction)
  (if (Variables|Default|GetIsMale)
    (Components|StaticMesh|SetStaticMesh (Variables|Default|GetAnimalMesh) "/Game/GameContent/Visuals/Characters/Animals/SM_BunnyMale.SM_BunnyMale")
    (else
      (Components|StaticMesh|SetStaticMesh (Variables|Default|GetAnimalMesh) "/Game/GameContent/Visuals/Characters/Animals/SM_BunnyFemale.SM_BunnyFemale"))))