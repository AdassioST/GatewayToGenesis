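; Base plant Blueprint that animals feed on by entering its interaction range, with a cooldown on feeding.
; An overlapping BP_BaseAnimal with a qualifying priority has its hunger decreased if the plant is off cooldown, then a timer triggers RefreshCooldown.
; RefreshCooldown decrements the cooldown or clears it, recoloring all point lights to show the state.
; Failed animal casts report to the player character's ErrorHandler.
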(event OnComponentBeginOverlap(InteractionRange)
  (params (OverlappedComponent :type Primitive%20Component%20Object%20Reference) (OtherActor :type Actor%20Object%20Reference) (OtherComp :type Primitive%20Component%20Object%20Reference) (OtherBodyIndex :type Integer) (bFromSweep :type Boolean) (SweepResult :type Hit%20Result%20Structure%20%28by%20ref%29))
  ;[1 1 1] Verificar que lo que esta tocando la planta es un animal, que el animal quiere comer y que este en enfriamiento la comida
  (if (== (Utilities|GetClass OtherActor) 0)
    (bind _asbp_base_animal (Utilities|Casting|CastToBP_BaseAnimal OtherActor)
      (:then
        (if (and (Utilities|Enum|NotEqual(Enum) (Variables|/Game/GameContent/Program/Characters/BP_BaseAnimal.BP_BaseAnimal_C|GetAnimalPriorities _asbp_base_animal) "NewEnumerator1") (not (Variables|Default|GetOnCooldown)))
          ;[1 1 1] Disminuir el hambre del animal y entrar en Cooldown
          (Default|DecreaseHunger _asbp_base_animal (Variables|Default|GetHungerRecovery))
          (Utilities|Time|SetTimerbyEvent (delegate Custom|RefreshCooldown) 1.0 (Variables|Default|GetOnCooldown))))
      (:CastFailed
        (Default|ErrorHandler (Variables|Default|GetCharacter%20Reference) self "Fallo el cast de BP_BaseAnimal")))))

(event Custom|RefreshCooldown
  ;[1 1 1] Disminuir el hambre del animal y entrar en Cooldown
  (if (> (Variables|Default|GetCooldown) 1.0)
    (Variables|Default|SetOnCooldown true)
    (Variables|Default|SetCooldown (- (Variables|Default|GetCooldown) 1.0))
    (Utilities|FlowControl|Delay 1.0)
    (Utilities|FlowControl|DoOnce false
      (:Completed
        (CallFunction|RefreshLightColor (Variables|Default|GetOnCooldownColor))))
    (else
      (Variables|Default|SetOnCooldown false)
      (CallFunction|RefreshLightColor (Variables|Default|GetOffCooldownColor)))))

(event EventBeginPlay
  (bind _asgg_my_character (Utilities|Casting|CastToGg_MyCharacter (Game|Player|GetPlayerPawn 0)))
  (Variables|Default|SetCharacter%20Reference _asgg_my_character))

(event Collision|EventActorBeginOverlap
  (params (OtherActor :type Actor%20Object%20Reference)))

(event EventTick
  (params (DeltaSeconds :type Float%20%28single-precision%29)))

(fn ConstructionScript)

(fn RefreshLightColor
  (params (LightColor :type Linear%20Color%20Structure))
  (for _array_element (Actor|GetComponentsByClass "/Script/Engine.PointLightComponent")
    (Rendering|Components|Light|SetLightColor _array_element LightColor true)))